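; BP_BattleRail_01 is an interactable animated rail prop in the BossMap folder.
; The first Interact call starts the rail animation looping on its skeletal mesh and sets HasPlayed.
; Later interactions set the animation's play rate to MultiplyRate rather than restarting it.
; Both paths print debug strings, and the construction script and other events are empty.
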(event EventBeginPlay)

(event Collision|EventActorBeginOverlap
  (params (OtherActor :type Actor%20Object%20Reference)))

(event EventTick
  (params (DeltaSeconds :type Float%20%28single-precision%29)))

(event EventInteract
  (params (Interactor :type Actor%20Object%20Reference))
  (if (Variables|Default|GetHasPlayed)
    (Components|Timeline|SetPlayRate (Variables|Default|GetSkeletalMesh) (Variables|Default|GetMultiplyRate))
    (Development|PrintString "2")
    (else
      (Components|Animation|PlayAnimation (Variables|Default|GetSkeletalMesh) "/Game/Maps/BossMap/Animation/SK_BF302_Rail_mo_Anim_SK_BF302_Rail_ao_A_BF302_Rail_01.SK_BF302_Rail_mo_Anim_SK_BF302_Rail_ao_A_BF302_Rail_01" true)
      (Variables|Default|SetHasPlayed true)
      (Utilities|FlowControl|DoOnce false
        (:Completed
          (Development|PrintString "Hello"))))))

(fn ConstructionScript)