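; BP_Tarminal is an interactable terminal that starts the transition from battle to the boss field.
; When the player enters its box, it enables input and shows the widget component's check popup labeled "보스필드" (boss field).
; Pressing Space, gated by a player cast on the overlapping actor, adds the transition widget and plays its animation.
; Any end overlap disables input and removes the popup.
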(event OnComponentBeginOverlap(Box)
  (params (OverlappedComponent :type Primitive%20Component%20Object%20Reference) (OtherActor :type Actor%20Object%20Reference) (OtherComp :type Primitive%20Component%20Object%20Reference) (OtherBodyIndex :type Integer) (bFromSweep :type Boolean) (SweepResult :type Hit%20Result%20Structure%20%28by%20ref%29))
  (Utilities|Casting|CastToBP_TPS_MainPlayer OtherActor)
  (Input|EnableInput (Game|GetPlayerController 0))
  (bind _aswbp_popup_check (Utilities|Casting|CastToWBP_Popup_CHECK (UserInterface|GetUserWidgetObject (Variables|Default|GetWidget))))
  (Variables|/Script/UMG.TextBlock|SetText (Variables|/Game/UI/Popup/WBP_Popup_CHECK.WBP_Popup_CHECK_C|GetTextBlock_38 _aswbp_popup_check) "보스필드")
  (Default|Create _aswbp_popup_check))

(event OnComponentEndOverlap(Box)
  (params (OverlappedComponent :type Primitive%20Component%20Object%20Reference) (OtherActor :type Actor%20Object%20Reference) (OtherComp :type Primitive%20Component%20Object%20Reference) (OtherBodyIndex :type Integer))
  (Input|DisableInput (Game|GetPlayerController 0))
  (bind _aswbp_popup_check (Utilities|Casting|CastToWBP_Popup_CHECK (UserInterface|GetUserWidgetObject (Variables|Default|GetWidget))))
  (Default|Remove _aswbp_popup_check))

(event EventBeginPlay)

(event Collision|EventActorBeginOverlap
  (params (OtherActor :type Actor%20Object%20Reference)))

(event EventTick
  (params (DeltaSeconds :type Float%20%28single-precision%29)))

(event Input|KeyboardEvents|SpaceBar
  (params (Key :type Key%20Structure :default "None"))
  (:Pressed
    (Utilities|Casting|CastToBP_TPS_MainPlayer (stale OnComponentBeginOverlap(Box) OtherActor))
    (bind _returnvalue (UserInterface|CreateWidget "/Game/UI/Transition/WBP_Trasition_BattleToBossField.WBP_Trasition_BattleToBossField_C"))
    (UserInterface|Viewport|AddtoViewport _returnvalue 0)
    (UserInterface|Animation|PlayAnimation _returnvalue (Variables|/Script/Persona3Reroad.TitleToLoadLevelWidget|GetCreateAnim _returnvalue) 0.0 1 "Forward" 1.0 false)))

(fn ConstructionScript)