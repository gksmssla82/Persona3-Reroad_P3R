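; BP_ItemBox3 is an openable treasure chest that updates the Battle04 box marker on the minimap.
; Player overlap with its Box enables actor input and shows a WBP_Popup_CHECK widget prompt, while end overlap reverses both.
; SpaceBar plays a sound and the open animation, then after a delay swaps the BP_MiniMap marker material to opened and disables Box collision.
; No item is granted in this graph.
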(event OnComponentBeginOverlap(Box)
  (params (OverlappedComponent :type Primitive%20Component%20Object%20Reference) (OtherActor :type Actor%20Object%20Reference) (OtherComp :type Primitive%20Component%20Object%20Reference) (OtherBodyIndex :type Integer) (bFromSweep :type Boolean) (SweepResult :type Hit%20Result%20Structure%20%28by%20ref%29))
  (Utilities|Casting|CastToBP_TPS_MainPlayer OtherActor)
  (Input|EnableInput (Game|GetPlayerController 0))
  (bind _aswbp_popup_check (Utilities|Casting|CastToWBP_Popup_CHECK (UserInterface|GetUserWidgetObject (Variables|Default|GetWidget))))
  (Variables|/Script/UMG.TextBlock|SetText (Variables|/Game/UI/Popup/WBP_Popup_CHECK.WBP_Popup_CHECK_C|GetTextBlock_38 _aswbp_popup_check) "보물상자")
  (Default|Create _aswbp_popup_check))

(event OnComponentEndOverlap(Box)
  (params (OverlappedComponent :type Primitive%20Component%20Object%20Reference) (OtherActor :type Actor%20Object%20Reference) (OtherComp :type Primitive%20Component%20Object%20Reference) (OtherBodyIndex :type Integer))
  (Input|DisableInput (Game|GetPlayerController 0))
  (bind _aswbp_popup_check (Utilities|Casting|CastToWBP_Popup_CHECK (UserInterface|GetUserWidgetObject (Variables|Default|GetWidget))))
  (Default|Remove _aswbp_popup_check))

(event EventBeginPlay)

(event Collision|EventActorBeginOverlap
  (params (OtherActor :type Actor%20Object%20Reference)))

(event EventTick
  (params (DeltaSeconds :type Float%20%28single-precision%29)))

(event Input|KeyboardEvents|SpaceBar
  (params (Key :type Key%20Structure :default "None"))
  (:Pressed
    (Audio|PlaySound2D "/Game/Sound/item.item" 1.0 1.0 0.0 0 0)
    (Components|Animation|PlayAnimation (Variables|Default|GetSkeletalMesh) "/Game/Maps/Item/SK_FLD_GimicBox_mo_Anim_SK_FLD_GimicBox_ao_A_FLD_GimicBox_Active.SK_FLD_GimicBox_mo_Anim_SK_FLD_GimicBox_ao_A_FLD_GimicBox_Active" false)
    (Utilities|FlowControl|Delay 1.0)
    (bind _returnvalue (Actor|GetActorOfClass "/Game/UI/MinMap/MinMpaWidget/Battle/BP_MiniMap.BP_MiniMap_C"))
    (Rendering|Material|SetMaterial (Variables|/Game/UI/MinMap/MinMpaWidget/Battle/BP_MiniMap.BP_MiniMap_C|GetBattle_04_Box _returnvalue) 0 "/Game/UI/MinMap/Battle/Matarial/MT_Battl_BoxOpen.MT_Battl_BoxOpen")
    (Collision|SetCollisionEnabled (Variables|Default|GetBox) "NoCollision")))

(fn ConstructionScript)