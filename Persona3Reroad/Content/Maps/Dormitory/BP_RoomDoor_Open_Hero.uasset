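; BP_RoomDoor_Open_Hero is a dormitory room door that sends the player to the hallway.
; Overlapping its box enables input and shows a WBP_Popup_GOTO widget labeled "복도" (hallway); leaving reverses both.
; Space starts the LS_dormitory_Open_Hero sequence and, without waiting for it, moves the BP_TPS_MainPlayer from the overlap to the Teleport location with a fixed yaw.
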(event OnComponentBeginOverlap(Box)
  (params (OverlappedComponent :type Primitive%20Component%20Object%20Reference) (OtherActor :type Actor%20Object%20Reference) (OtherComp :type Primitive%20Component%20Object%20Reference) (OtherBodyIndex :type Integer) (bFromSweep :type Boolean) (SweepResult :type Hit%20Result%20Structure%20%28by%20ref%29))
  (Input|EnableInput (Game|GetPlayerController 0))
  (bind _aswbp_popup_goto (Utilities|Casting|CastToWBP_Popup_GOTO (UserInterface|GetUserWidgetObject (Variables|Default|GetWidget))))
  (Variables|/Script/UMG.TextBlock|SetText (Variables|/Game/UI/Popup/WBP_Popup_GOTO.WBP_Popup_GOTO_C|GetTextBlock_38 _aswbp_popup_goto) "복도")
  (Default|Create _aswbp_popup_goto))

(event OnComponentEndOverlap(Box)
  (params (OverlappedComponent :type Primitive%20Component%20Object%20Reference) (OtherActor :type Actor%20Object%20Reference) (OtherComp :type Primitive%20Component%20Object%20Reference) (OtherBodyIndex :type Integer))
  (Input|DisableInput (Game|GetPlayerController 0))
  (bind _aswbp_popup_goto (Utilities|Casting|CastToWBP_Popup_GOTO (UserInterface|GetUserWidgetObject (Variables|Default|GetWidget))))
  (Default|Remove _aswbp_popup_goto))

(event EventBeginPlay
  (|CallParentFunction) ; This node is disabled and will not be called.\nDrag off pins to build functionality.
)

(event Collision|EventActorBeginOverlap
  (params (OtherActor :type Actor%20Object%20Reference))
  (|CallParentFunction OtherActor) ; This node is disabled and will not be called.\nDrag off pins to build functionality.
)

(event EventTick
  (params (DeltaSeconds :type Float%20%28single-precision%29))
  (|CallParentFunction DeltaSeconds) ; This node is disabled and will not be called.\nDrag off pins to build functionality.
)

(event Input|KeyboardEvents|SpaceBar
  (params (Key :type Key%20Structure :default "None"))
  (:Pressed
    (bind _returnvalue (Sequencer|Player|CreateLevelSequencePlayer "/Game/Sequences/LS_dormitory_Open_Hero.LS_dormitory_Open_Hero"))
    (Sequencer|Player|Play _returnvalue :!class /Script/MovieScene.MovieSceneSequencePlayer)
    (bind _asbp_tps_main_player (Utilities|Casting|CastToBP_TPS_MainPlayer (stale OnComponentBeginOverlap(Box) OtherActor)))
    (Transformation|SetActorLocation _asbp_tps_main_player (Transformation|GetActorLocation (Variables|Default|GetTeleport)) false false)
    (Transformation|SetActorRotation _asbp_tps_main_player (Math|Rotator|MakeRotator 0.0 0.0 9e+01))))

(fn ConstructionScript
  (|CallParentFunction))