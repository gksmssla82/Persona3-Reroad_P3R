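; Trigger-box actor that shows the Dormitory 2F widget, a minimap going by the asset name, while something overlaps its Box.
; Begin overlap waits briefly, then creates WBP_2F_Dormitory, stores it, adds it to the viewport and plays ScreenIn.
; End overlap starts ScreenOut and removes the stored widget immediately, without waiting for the animation.
; Neither event filters the overlapping actor or cancels the pending delay.
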(event OnComponentBeginOverlap(Box)
  (params (OverlappedComponent :type Primitive%20Component%20Object%20Reference) (OtherActor :type Actor%20Object%20Reference) (OtherComp :type Primitive%20Component%20Object%20Reference) (OtherBodyIndex :type Integer) (bFromSweep :type Boolean) (SweepResult :type Hit%20Result%20Structure%20%28by%20ref%29))
  (Utilities|FlowControl|Delay 1.567)
  (bind _returnvalue (UserInterface|CreateWidget "/Game/UI/MinMap/MinMpaWidget/Dormitory/WBP_2F_Dormitory.WBP_2F_Dormitory_C"))
  (Variables|Default|Set2FDormitory _returnvalue)
  (UserInterface|Viewport|AddtoViewport _returnvalue 0)
  (UserInterface|Animation|PlayAnimation _returnvalue (Variables|/Script/Persona3Reroad.BaseMiniMapWidget|GetScreenIn _returnvalue) 0.0 1 "Forward" 1.0 false))

(event OnComponentEndOverlap(Box)
  (params (OverlappedComponent :type Primitive%20Component%20Object%20Reference) (OtherActor :type Actor%20Object%20Reference) (OtherComp :type Primitive%20Component%20Object%20Reference) (OtherBodyIndex :type Integer))
  (bind _2fdormitory (Variables|Default|Get2FDormitory))
  (UserInterface|Animation|PlayAnimation _2fdormitory (Variables|/Script/Persona3Reroad.BaseMiniMapWidget|GetScreenOut _2fdormitory) 0.0 1 "Forward" 1.0 false)
  (Widget|RemovefromParent (Variables|Default|Get2FDormitory)))

(event EventBeginPlay)

(event Collision|EventActorBeginOverlap
  (params (OtherActor :type Actor%20Object%20Reference)))

(event EventTick
  (params (DeltaSeconds :type Float%20%28single-precision%29)))

(fn ConstructionScript)