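; Base game mode for a Persona-style game that sets up the level's HUD through a widget instance subsystem.
; BeginPlay creates the widgets and target controller, then queues the battle minimap and day widgets, looked up by tag from a registry map.
; Tick waits until the battle subsystem's player party holds four members, then queues the field party panel and adds the level's widgets to the viewport, guarded by a one-shot flag.
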(event EventBeginPlay
  (bind _returnvalue (Subsystems|GetWidgetInstanceSubsystem))
  (Class|WidgetInstanceSubsystem|CreateWidget _returnvalue)
  (Class|WidgetInstanceSubsystem|CreateTargetController _returnvalue)
  (Class|WidgetInstanceSubsystem|AddfromCurrenLevelWidgetArray _returnvalue (Class|WidgetInstanceSubsystem|FindRegistryWidgetMap _returnvalue "(TagName=\"Widget.MiniMap.BattleMiniMap\")"))
  (Class|WidgetInstanceSubsystem|AddfromCurrenLevelWidgetArray _returnvalue (Class|WidgetInstanceSubsystem|FindRegistryWidgetMap _returnvalue "(TagName=\"Widget.Global.Day\")")))

(event EventTick
  (params (DeltaSeconds :type Float%20%28single-precision%29))
  (bind _returnvalue (Subsystems|GetWidgetInstanceSubsystem))
  (if (and (== (Utilities|Array|Length (Variables|/Script/Persona3Reroad.BattleInstanceSubsystem|GetPlayerParty (Subsystems|GetBattleInstanceSubsystem))) 4) (Variables|Default|GetTBCLoadCheck))
    (Class|WidgetInstanceSubsystem|AddfromCurrenLevelWidgetArray _returnvalue (Class|WidgetInstanceSubsystem|FindRegistryWidgetMap _returnvalue "(TagName=\"Widget.Battle.PartyPanel.Field\")"))
    (Variables|Default|SetTBCLoadCheck false)
    (Class|WidgetInstanceSubsystem|AddViewportEventCurrentLevelWidgetArray (Subsystems|GetWidgetInstanceSubsystem))))

(fn ConstructionScript)