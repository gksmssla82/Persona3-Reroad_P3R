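; Third-person player character Blueprint that handles melee attack input.
; IA_Attack plays a standing or sprint-dash attack montage based on IsSprint, using IsAttack to block re-entry until it completes or is interrupted, then resetting MoveSpeed.
; A debug H key adds the battle party panel widget to the viewport through the widget instance subsystem's registry.
; BeginPlay and the weapon collider overlap event are empty.
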(event OnComponentBeginOverlap(WeaponColider)
  (params (OverlappedComponent :type Primitive%20Component%20Object%20Reference) (OtherActor :type Actor%20Object%20Reference) (OtherComp :type Primitive%20Component%20Object%20Reference) (OtherBodyIndex :type Integer) (bFromSweep :type Boolean) (SweepResult :type Hit%20Result%20Structure%20%28by%20ref%29)))

(event Input|EnhancedActionEvents|EnhancedInputActionIA_Attack
  (params (ActionValue :type Boolean) (ElapsedSeconds :type Float%20%28double-precision%29) (TriggeredSeconds :type Float%20%28double-precision%29) (InputAction :type Input%20Action%20Object%20Reference :default "/Game/BP/Input/IA_Attack.IA_Attack"))
  (:Started
    (if (not (Variables|Default|GetIsAttack))
      (Variables|Default|SetIsAttack true)
      (if (not (Variables|Default|GetIsSprint))
        (Animation|Montage|PlayMontage (Variables|Character|GetMesh) "/Game/BP/Character/TPS/Player/Anim/Montage/A_PC0001_DNG0015_BASE_AttackA_Montage.A_PC0001_DNG0015_BASE_AttackA_Montage"
          (:OnCompleted
            _)
          (:OnInterrupted
            _))
        (Variables|Default|SetIsAttack false)
        (Variables|Default|SetMoveSpeed 2e+02)
        (else
          (Animation|Montage|PlayMontage (Variables|Character|GetMesh) "/Game/BP/Character/TPS/Player/Anim/Montage/A_PC0001_DNG0016_BASE_AttackDashA_Montage.A_PC0001_DNG0016_BASE_AttackDashA_Montage"
            (:OnCompleted
              _)
            (:OnInterrupted
              _))
          (Variables|Default|SetIsAttack false)
          (Variables|Default|SetMoveSpeed 2e+02))))))

(event EventBeginPlay)

(event Input|KeyboardEvents|DebugKeyH
  (params (Key :type Key%20Structure :default "None") (ActionValue :type Input%20Action%20Value%20Structure))
  (:Pressed
    (Class|BaseUIWidget|AddViewportEvent (Class|WidgetInstanceSubsystem|FindRegistryWidgetMap (Subsystems|GetWidgetInstanceSubsystem) "(TagName=\"Widget.Battle.PartyPanel.Battle\")"))
    (Development|PrintString "Hello")))

(fn ConstructionScript)