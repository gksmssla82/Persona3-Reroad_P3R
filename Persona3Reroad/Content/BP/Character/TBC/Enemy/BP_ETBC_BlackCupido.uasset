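; BlackCupido enemy Blueprint for turn-based combat.
; On BeginPlay it calls the parent logic, then registers the MahaKouga and Gal skills on itself through the BattleSkillManager of the BattleInstanceSubsystem.
; The overlap and Tick events are disabled, and the construction script only calls its parent.
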(event EventBeginPlay
  (bind _returnvalue (Subsystems|GetBattleInstanceSubsystem))
  (bind _battleskillmanager (Variables|/Script/Persona3Reroad.BattleInstanceSubsystem|GetBattleSkillManager _returnvalue))
  (|CallParentFunction)
  (Class|SkillManager|AddSkill _battleskillmanager "MahaKouga" self 0)
  (Class|SkillManager|AddSkill _battleskillmanager "Gal" self 0))

(event Collision|EventActorBeginOverlap
  (params (OtherActor :type Actor%20Object%20Reference))
  (|CallParentFunction OtherActor) ; This node is disabled and will not be called.\nDrag off pins to build functionality.
)

(event EventTick
  (params (DeltaSeconds :type Float%20%28single-precision%29))
  (|CallParentFunction DeltaSeconds) ; This node is disabled and will not be called.\nDrag off pins to build functionality.
)

(fn ConstructionScript
  (|CallParentFunction))