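; Persona Blueprint for Io in the turn-based battle system, which registers this persona's skill set.
; On BeginPlay, after the parent logic, it adds Booh, Kouha and MahaBoohra by name to the battle instance subsystem's BattleSkillManager, passing itself as the owning persona.
; It has no other active logic of its own, as Tick and overlap are disabled and construction only calls the parent.
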(event EventBeginPlay
  (bind _returnvalue (Subsystems|GetBattleInstanceSubsystem))
  (bind _battleskillmanager (Variables|/Script/Persona3Reroad.BattleInstanceSubsystem|GetBattleSkillManager _returnvalue))
  (|CallParentFunction)
  (Class|SkillManager|AddSkill (Variables|/Script/Persona3Reroad.BattleInstanceSubsystem|GetBattleSkillManager (Subsystems|GetBattleInstanceSubsystem)) "Booh" 0 self)
  (Class|SkillManager|AddSkill _battleskillmanager "Kouha" 0 self)
  (Class|SkillManager|AddSkill _battleskillmanager "MahaBoohra" 0 self))

(event Collision|EventActorBeginOverlap
  (params (OtherActor :type Actor%20Object%20Reference))
  (|CallParentFunction OtherActor) ; This node is disabled and will not be called.\nDrag off pins to build functionality.
)

(event EventTick
  (params (DeltaSeconds :type Float%20%28single-precision%29))
  (|CallParentFunction DeltaSeconds) ; This node is disabled and will not be called.\nDrag off pins to build functionality.
)

(fn ConstructionScript
  (|CallParentFunction))