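; Penthesilea Persona Blueprint for turn-based combat that supplies the Persona's battle skill set.
; On BeginPlay it runs the parent logic, then registers its light and electric skills (Kouha, Zio and their Maha variants) by name with the BattleInstanceSubsystem's BattleSkillManager, passing itself as the PersonaSkill.
; All other behavior comes from the parent class, as the overlap and tick events are disabled.
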(event EventBeginPlay
  (bind _returnvalue (Subsystems|GetBattleInstanceSubsystem))
  (bind _self self)
  (bind _battleskillmanager (Variables|/Script/Persona3Reroad.BattleInstanceSubsystem|GetBattleSkillManager _returnvalue))
  (|CallParentFunction)
  (Class|SkillManager|AddSkill (Variables|/Script/Persona3Reroad.BattleInstanceSubsystem|GetBattleSkillManager (Subsystems|GetBattleInstanceSubsystem)) "Kouha" 0 self)
  (Class|SkillManager|AddSkill _battleskillmanager "Zio" 0 _self)
  (Class|SkillManager|AddSkill _battleskillmanager "MahaKouga" 0 _self)
  (Class|SkillManager|AddSkill _battleskillmanager "MahaZio" 0 _self))

(event Collision|EventActorBeginOverlap
  (params (OtherActor :type Actor%20Object%20Reference))
  (|CallParentFunction OtherActor) ; This node is disabled and will not be called.\nDrag off pins to build functionality.
)

(event EventTick
  (params (DeltaSeconds :type Float%20%28single-precision%29))
  (|CallParentFunction DeltaSeconds) ; This node is disabled and will not be called.\nDrag off pins to build functionality.
)

(fn ConstructionScript
  (|CallParentFunction))