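; Player character Blueprint for Yukari, apparently for turn-based combat (TBC), that sets up her battle skill and cut-in movie.
; On BeginPlay it runs the parent logic, then registers the "Shot" skill on itself through the battle instance subsystem's skill manager.
; It then immediately opens the PC0002 battle cut-in media source and plays it.
; Tick and overlap events are disabled stubs, and construction only calls the parent.
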(event EventBeginPlay
  (bind _target (Variables|Default|GetTarget))
  (|CallParentFunction)
  (Class|SkillManager|AddSkill (Variables|/Script/Persona3Reroad.BattleInstanceSubsystem|GetBattleSkillManager (Subsystems|GetBattleInstanceSubsystem)) "Shot" self 0)
  (Media|MediaPlayer|OpenSource _target "/Game/Cutin/MS_Btl_Cutin_PC0002_VP9_converted.MS_Btl_Cutin_PC0002_VP9_converted")
  (Media|MediaPlayer|Play _target :!class /Script/MediaAssets.MediaPlayer))

(event Collision|EventActorBeginOverlap
  (params (OtherActor :type Actor%20Object%20Reference))
  (|CallParentFunction OtherActor) ; This node is disabled and will not be called.\nDrag off pins to build functionality.
)

(event EventTick
  (params (DeltaSeconds :type Float%20%28single-precision%29))
  (|CallParentFunction DeltaSeconds) ; This node is disabled and will not be called.\nDrag off pins to build functionality.
)

(fn ConstructionScript
  (|CallParentFunction))