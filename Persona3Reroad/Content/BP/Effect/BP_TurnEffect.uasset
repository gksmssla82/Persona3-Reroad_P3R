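; BP_TurnEffect is a turn-based effect that modifies a named attribute on a target component, such as its min, max or current value.
; ApplyEffect runs DoEffect by effect type: instant, for a turn count, infinite or temporary.
; CalculateNewValue adds, multiplies, divides or overrides, recording the change so EndEffect can reverse temporary effects before removing itself from ActiveEffects.
; The Current Value Mod case writes its result into CurrentValue.
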(event Custom|ApplyEffect
  (switch Utilities|FlowControl|Switch|SwitchonEEffectType (Variables|Default|GetEffectType)
    (:Instant
      (CallFunction|DoEffect)
      (CallFunction|EndEffect))
    (:forTurns
      (CallFunction|DoEffect)
      (bind _result (Math|Integer|DecrementInt (Variables|Default|GetEffectTurnCounter))
        (:%20%20
          (if (<= _result 0)
            (CallFunction|EndEffect)))))
    (:Infinite
      (CallFunction|DoEffect))
    (:Temporary
      (CallFunction|DoEffect))))

(event Custom|EndEffect
  (switch Utilities|FlowControl|Switch|SwitchonEEffectType (Variables|Default|GetEffectType)
    (:Instant
      _)
    (:forTurns
      _)
    (:Infinite
      _)
    (:Temporary
      (Variables|Default|SetEffectMath "Add")
      (Variables|Default|SetMagnitude (* (Variables|Default|GetAbsoluteChange) -1.0))
      (CallFunction|DoEffect)))
  (Utilities|Array|RemoveItem (Variables|/Game/BP/Effect/MyTurnBaseAbilityComponent.MyTurnBaseAbilityComponent_C|GetActiveEffects (Variables|Default|GetTargetComponent)) self))

(fn DoEffect
  (bind _targetcomponent (Variables|Default|GetTargetComponent)
    (:then
      (for (_array_element _array_index) (Variables|/Script/Persona3Reroad.TurnBaseAbilityComponent|GetAttributes _targetcomponent)
        (if (== (.name _array_element) (Variables|Default|GetAttributeToEffect))
          (switch Utilities|FlowControl|Switch|SwitchonETargetStat (Variables|Default|GetTargetStat)
            (:MinValue
              (bind _returnvalue (CallFunction|CalculateNewValue (.MinValue (Utilities|Struct|BreakStat (.Stat (Utilities|Struct|BreakTurnBaseAttribute (Utilities|Array|Get(acopy) (Variables|/Script/Persona3Reroad.TurnBaseAbilityComponent|GetAttributes _targetcomponent) _array_index)))))))
              (Utilities|Struct|SetmembersinStat (.Stat (Utilities|Struct|BreakTurnBaseAttribute (Utilities|Array|Get(acopy) (Variables|/Script/Persona3Reroad.TurnBaseAbilityComponent|GetAttributes _targetcomponent) _array_index))) _returnvalue))
            (:MinValueMod
              (bind _returnvalue_2 (CallFunction|CalculateNewValue (.MinValueMod (Utilities|Struct|BreakStat (.Stat (Utilities|Struct|BreakTurnBaseAttribute (Utilities|Array|Get(acopy) (Variables|/Script/Persona3Reroad.TurnBaseAbilityComponent|GetAttributes _targetcomponent) _array_index)))))))
              (Utilities|Struct|SetmembersinStat (.Stat (Utilities|Struct|BreakTurnBaseAttribute (Utilities|Array|Get(acopy) (Variables|/Script/Persona3Reroad.TurnBaseAbilityComponent|GetAttributes _targetcomponent) _array_index))) _returnvalue_2))
            (:MaxValue
              (bind _returnvalue_3 (CallFunction|CalculateNewValue (.MaxValue (Utilities|Struct|BreakStat (.Stat (Utilities|Struct|BreakTurnBaseAttribute (Utilities|Array|Get(acopy) (Variables|/Script/Persona3Reroad.TurnBaseAbilityComponent|GetAttributes _targetcomponent) _array_index)))))))
              (Utilities|Struct|SetmembersinStat (.Stat (Utilities|Struct|BreakTurnBaseAttribute (Utilities|Array|Get(acopy) (Variables|/Script/Persona3Reroad.TurnBaseAbilityComponent|GetAttributes _targetcomponent) _array_index))) _returnvalue_3))
            (:MaxValueMod
              (bind _returnvalue_4 (CallFunction|CalculateNewValue (.MaxValueMod (Utilities|Struct|BreakStat (.Stat (Utilities|Struct|BreakTurnBaseAttribute (Utilities|Array|Get(acopy) (Variables|/Script/Persona3Reroad.TurnBaseAbilityComponent|GetAttributes _targetcomponent) _array_index)))))))
              (Utilities|Struct|SetmembersinStat (.Stat (Utilities|Struct|BreakTurnBaseAttribute (Utilities|Array|Get(acopy) (Variables|/Script/Persona3Reroad.TurnBaseAbilityComponent|GetAttributes _targetcomponent) _array_index))) _returnvalue_4))
            (:CurrentValue
              (bind _returnvalue_5 (CallFunction|CalculateNewValue (.CurrentValue (Utilities|Struct|BreakStat (.Stat (Utilities|Struct|BreakTurnBaseAttribute (Utilities|Array|Get(acopy) (Variables|/Script/Persona3Reroad.TurnBaseAbilityComponent|GetAttributes _targetcomponent) _array_index)))))))
              (Utilities|Struct|SetmembersinStat (.Stat (Utilities|Struct|BreakTurnBaseAttribute (Utilities|Array|Get(acopy) (Variables|/Script/Persona3Reroad.TurnBaseAbilityComponent|GetAttributes _targetcomponent) _array_index))) (Math|Float|Clamp(Float) _returnvalue_5 (stale _returnvalue_7) (stale _returnvalue_8))))
            (:CurrentValueMod
              (bind _returnvalue_6 (CallFunction|CalculateNewValue (.CurrentValueMod (Utilities|Struct|BreakStat (.Stat (Utilities|Struct|BreakTurnBaseAttribute (Utilities|Array|Get(acopy) (Variables|/Script/Persona3Reroad.TurnBaseAbilityComponent|GetAttributes _targetcomponent) _array_index)))))))
              (bind _returnvalue_7 (Class|TurnBaseAbilityComponent|GetAttributeMin (Variables|Default|GetTargetComponent) (Variables|Default|GetAttributeToEffect)))
              (bind _returnvalue_8 (Class|TurnBaseAbilityComponent|GetAttributeMax (Variables|Default|GetTargetComponent) (Variables|Default|GetAttributeToEffect)))
              (Utilities|Struct|SetmembersinStat (.Stat (Utilities|Struct|BreakTurnBaseAttribute (Utilities|Array|Get(acopy) (Variables|/Script/Persona3Reroad.TurnBaseAbilityComponent|GetAttributes _targetcomponent) _array_index))) _returnvalue_6)))
          (Default|CallUpdateAttribute (Utilities|Array|Get(acopy) (Variables|/Script/Persona3Reroad.TurnBaseAbilityComponent|GetAttributes _targetcomponent) _array_index))
          (return))))
    (:else)))

(fn CalculateNewValue
  (params (OldValue :type Float%20%28double-precision%29))
  (bind _magnitude (Variables|Default|GetMagnitude))
  (bind _magnitude_2 (Variables|Default|GetMagnitude))
  (bind _magnitude_3 (Variables|Default|GetMagnitude))
  (bind _magnitude_4 (Variables|Default|GetMagnitude))
  (bind _returnvalue (+ _magnitude_2 OldValue))
  (bind _returnvalue_2 (* _magnitude_3 OldValue))
  (bind _returnvalue_3 (/ _magnitude_4 OldValue))
  (switch Utilities|FlowControl|Switch|SwitchonEEffectMath (Variables|Default|GetEffectMath)
    (:Add
      (Variables|Default|SetAbsoluteChange (- _returnvalue OldValue))
      (return _returnvalue))
    (:Mulitply
      (Variables|Default|SetAbsoluteChange (- _returnvalue_2 OldValue))
      (return _returnvalue_2))
    (:Divide
      (Variables|Default|SetAbsoluteChange (- _returnvalue_3 OldValue))
      (return _returnvalue_3))
    (:Override
      (Variables|Default|SetAbsoluteChange (- _magnitude OldValue))
      (return _magnitude))))